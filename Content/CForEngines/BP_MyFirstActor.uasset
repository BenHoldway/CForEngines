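; BP_MyFirstActor is an actor that plays a hi-hat sound as a metronome-like beat using Quartz.
; On BeginPlay it creates a 4/4 Quartz clock at 180 BPM, subscribes HiHat to quarter-note quantization, and starts the clock.
; Each quantization event calls PlaySound2D directly rather than scheduling quantized playback.
; Unconnected ApplyDamage and GetHandleForClock nodes never run.
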(event Custom|HiHat
  (params (ClockName :type Name) (QuantizationType :type EQuartzCommandQuantization%20Enum :default "Bar") (NumBars :type Integer) (Beat :type Integer) (BeatFraction :type Float%20%28single-precision%29))
  (Audio|PlaySound2D "/Game/HiHat.HiHat" 1.0 1.0 0.0 0 0))

(event EventBeginPlay
  (bind _returnvalue (Class|QuartzSubsystem|CreateNewClock (WorldSubsystems|GetQuartzSubsystem) "Fuck" (Utilities|Struct|MakeQuartzClockSettings (Utilities|Struct|MakeQuartzTimeSignature 4 "QuarterNote") false) false))
  (bind _clockhandle (Class|QuartzClockHandle|SetBeatsPerMinute :self _returnvalue :BeatsPerMinute 1.8e+02))
  (bind _output_get (Variables|Default|SetQuartzClock _clockhandle))
  (bind _clockhandle_2 (Class|QuartzClockHandle|SubscribetoQuantizationEvent _output_get "QuarterNote" (delegate Custom|HiHat)))
  (Class|QuartzClockHandle|StartClock _clockhandle_2))

(event Input|KeyboardEvents|F
  (params (Key :type Key%20Structure)))

(fn ConstructionScript)